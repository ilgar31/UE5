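; BP_Hero is the player hero character, moving on the world X/Y plane and facing left or right with its travel.
; The left/right and up/down input axes feed half-strength movement input along world X and Y.
; Each tick, the sign of X velocity sets the controller's rotation to zero or a 180-degree pitch (not yaw) flip, leaving it unchanged at zero velocity.
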(event EventTick
  (params (DeltaSeconds :type Float%20%28single-precision%29))
  (bind _returnvalue (Pawn|GetController))
  (bind _returnvalue_2 (Pawn|GetController))
  (Math|Float|CompareFloat (.x (Variables|/Script/Engine.MovementComponent|GetVelocity (Variables|Character|GetCharacterMovement))) 0.0
    (:>
      (Utilities|IsValid _returnvalue
        (:Is%20Valid
          (Pawn|SetControlRotation _returnvalue (Math|Rotator|MakeRotator 0.0 0.0 0.0)))))
    (:<
      (Utilities|IsValid _returnvalue_2
        (:Is%20Valid
          (Pawn|SetControlRotation _returnvalue_2 (Math|Rotator|MakeRotator 0.0 1.8e+02 0.0)))))))

(event Input|AxisEvents|InputAxismoveleft/right
  (params (AxisValue :type Float%20%28single-precision%29))
  (Pawn|Input|AddMovementInput "0.500000,0.000000,0.000000" AxisValue false))

(event Input|AxisEvents|InputAxismoveup/botton
  (params (AxisValue :type Float%20%28single-precision%29))
  (Pawn|Input|AddMovementInput "0.000000,0.500000,0.000000" AxisValue false))

(fn ConstructionScript)